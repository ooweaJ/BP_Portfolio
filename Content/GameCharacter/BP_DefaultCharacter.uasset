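; BP_DefaultCharacter is a character Blueprint that handles incoming damage and exposes combat stats through a StatusComponent.
; AnyDamage calls SetDamage, which, given a valid instigator, lowers health by defense-mitigated damage on a diminishing-returns curve and records the causer and attacking character.
; It then sends a DeBuffMessage to the DamageType with itself as target.
; OwnerInfo returns attack power, critical and attack speed, while GetTriggerEffect is an empty stub.
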(event `self.ReceiveAnyDamage`
  (params (Damage :type "Float (single-precision)") (DamageType :type "DamageType Object Reference") (InstigatedBy :type "Controller Object Reference") (DamageCauser :type "Actor Object Reference"))
  (`self.SetDamage` InstigatedBy DamageCauser Damage DamageType)
  (message `/Game/Office/Interfaces/IDamageType.DeBuff` DamageType "NewEnumerator0" "NewEnumerator0" self))

(fn `Defense Damage`
  (params (InDamage :type "Float (double-precision)"))
  (returns (ReturnDamage :type "Float (double-precision)"))
  (bind _indamage (`local.InDamage`))
  (bind _defense (`/Game/Office/Component/StatusComponent.Defense` (`self.StatusComponent`)))
  (return (- _indamage (* _indamage (/ _defense (+ _defense 100.0))))))

(fn `GetTriggerEffect`
  (params (Effcet :type "/Game/Office/Enum/EEffect Enum" :default "NewEnumerator0")))

(fn `OwnerInfo`
  (returns (AttackPower :type "Float (double-precision)") (Critical :type "Float (double-precision)") (AttackSpeed :type "Float (double-precision)"))
  (bind (_attackpower _critical _attackspeed) (`/Game/Office/Component/StatusComponent.GetInfo` (`self.StatusComponent`)))
  (return _attackpower _critical _attackspeed))

(fn `SetDamage`
  (params (Controller :type "Controller Object Reference") (Causer :type "Actor Object Reference") (Damage :type "Float (double-precision)") (DamageType :type "DamageType Object Reference"))
  (`/Engine/EditorBlueprintResources/StandardMacros.IsValid` Controller
    (:`Is Valid`
      (bind _returndamage (`self.Defense Damage` (`local.Damage`)))
      (`/Game/Office/Component/StatusComponent.SetDecreaseInfo` (`self.StatusComponent`) 0.0 0.0 0.0 0.0 0.0 _returndamage)
      (set `self.Causer` Causer)
      (bind _asbp_default_character (cast `/Game/GameCharacter/BP_DefaultCharacter` (`Controller.K2_GetPawn` Controller)))
      (set `self.Attacker` _asbp_default_character))))

(fn `UserConstructionScript`)