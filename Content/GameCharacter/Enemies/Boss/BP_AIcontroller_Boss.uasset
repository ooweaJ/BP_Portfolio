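; AI controller for the boss enemy that runs the possessed pawn's behavior tree and tracks the player through perception.
; On possess, it casts the pawn to BP_Enemy_AI, stores it, and starts that pawn's BehaivorTree if valid.
; Each perception update scans perceived actors for BP_Player, writes it to the PlayerKey blackboard entry and breaks the loop through a custom event, or clears the key when none is found.
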(event `self.ReceivePossess`
  (params (PossessedPawn :type "Pawn Object Reference"))
  (bind _asbp_enemy_ai (cast `/Game/GameCharacter/Enemies/EnemyAI/BP_Enemy_AI` PossessedPawn))
  (bind _output_get (set `self.AIPawn` _asbp_enemy_ai))
  (bind _behaivortree (`/Game/GameCharacter/Enemies/EnemyAI/BP_Enemy_AI.BehaivorTree` _output_get)
    (:`then`
      (`self.RunBehaviorTree` _behaivortree))
    (:`else`)))

(event `self.AIPerception.OnPerceptionUpdated`
  (params (UpdatedActors :type "Array of Actor Object Reference (by ref)"))
  (set `self.FinePlayer` false)
  (for _array_element (`AIPerceptionComponent.GetCurrentlyPerceivedActors` (`self.AIPerception`) null) :!label _label
    (bind _asbp_player (cast `/Game/GameCharacter/Player/BP_Player` _array_element))
    (`BlackboardComponent.SetValueAsObject` (`AIBlueprintHelperLibrary.GetBlackboard` null) "PlayerKey" _asbp_player)
    (set `self.FinePlayer` true)
    (`self.PerceptionBreak`))
  (if (not (`self.FinePlayer`))
    (`BlackboardComponent.SetValueAsObject` (`AIBlueprintHelperLibrary.GetBlackboard` null) "PlayerKey" null)))

(event `PerceptionBreak`
  (goto _label :!via `Break`))

(fn `UserConstructionScript`)