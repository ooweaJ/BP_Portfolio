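; Boss enemy character that spawns and attaches its own weapon, provides special attacks, and tracks idle/action state.
; Approach leaps at the player by turning a predicted projectile arc into a detached spline, which a timeline moves the boss along.
; SpawnKnife uses a delayed-loop macro to spawn swords one by one along a second spline, aimed by a boss-to-player rotation.
; FlyMoveAttack sphere-traces for player characters, damaging and launching them upward.
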(event `self.ReceiveBeginPlay`
  (`parent.ReceiveBeginPlay`)
  (bind _returnvalue (`|SpawnActorFromClass` "/Game/Item/Equipment/BP_BossWeapon.BP_BossWeapon_C" (`self.GetTransform`) "Undefined" "OverrideRootScale" self null))
  (bind _output_get (set `self.BossWeapon` _returnvalue))
  (`self.K2_AttachToComponent` _output_get (`self.Mesh`) "None" "KeepRelative" "KeepRelative" "KeepRelative" true))

(event `Approach`
  (params (PlayerLocation :type "Vector Structure"))
  (bind _outlaunchvelocity (`GameplayStatics.SuggestProjectileVelocity_CustomArc` (`self.K2_GetActorLocation`) PlayerLocation))
  (bind (_outhit _outpathpositions) (`GameplayStatics.Blueprint_PredictProjectilePath_ByObjectType` (`self.K2_GetActorLocation`) _outlaunchvelocity true 10.0 (`|MakeArray` "ObjectTypeQuery3" :!type "EObjectTypeQuery Enum") false (`|MakeArray` self :!type "Actor Object Reference") "ForDuration" 5.0 30.0 5.0))
  (`SplineComponent.SetSplinePoints` (`self.Spline`) _outpathpositions "World" true)
  (`SceneComponent.K2_DetachFromComponent` (`self.Spline`) "KeepWorld" "KeepWorld" "KeepWorld" true)
  (bind (_direction `_새_트랙_0`) (`Timeline|타임라인_0` :!via `PlayFromStart`)
    (:`Update`
      (`self.K2_SetActorLocation` (`SplineComponent.GetLocationAtDistanceAlongSpline` (`self.Spline`) (`KismetMathLibrary.Lerp` 0.0 (`SplineComponent.GetSplineLength` (`self.Spline`)) `_새_트랙_0`) "World")))))

(event `SpawnKnife`
  (params (PlayerKey :type "Vector Structure"))
  (bind _spline1 (`self.Spline1`))
  (bind _index (`self.For Loop Delay` 0 (`KismetMathLibrary.FFloor` (/ (`SplineComponent.GetSplineLength` _spline1) 50.0)) 0.2)
    (:`Loop Body`
      (`|SpawnActorFromClass` "/Game/Item/BossSword.BossSword_C" (`KismetMathLibrary.MakeTransform` (`SplineComponent.GetLocationAtDistanceAlongSpline` _spline1 (* _index 50.0) "World") (`KismetMathLibrary.FindLookAtRotation` (`self.K2_GetActorLocation`) PlayerKey) (0.5 0.5 0.5)) "Undefined" "OverrideRootScale" self null))))

(event `FlyMoveAttack`
  (bind _returnvalue (`SceneComponent.GetSocketLocation` (`self.Mesh`) "None"))
  (bind _outhits (`KismetSystemLibrary.SphereTraceMultiForObjects` _returnvalue _returnvalue 300.0 (`|MakeArray` "ObjectTypeQuery3" :!type "EObjectTypeQuery Enum")))
  (for _array_element _outhits
    (bind (_bblockinghit _binitialoverlap _time _distance _location _impactpoint _normal _impactnormal _physmat _hitactor) (`GameplayStatics.BreakHitResult` _array_element))
    (if (!= _hitactor self)
      (bind _asbp_default_character (cast `/Game/GameCharacter/BP_DefaultCharacter` _hitactor))
      (`GameplayStatics.ApplyDamage` _asbp_default_character 100.0 (`self.GetController`) self)
      (`self.LaunchCharacter` _asbp_default_character (0.0 0.0 1000.0) false false))))

(fn `FlyAttack`
  (params (PlayerLocation :type "Vector Structure")))

(fn `Get Current Item`
  (returns (`Current Item` :type "/Game/Item/BP_Item Object Reference"))
  (return (`self.BossWeapon`)))

(fn `Get Equip Item`
  (returns (`Equip Item` :type "/Game/Office/Enum/EItemType Enum"))
  (return "NewEnumerator1"))

(fn `Is State Action`
  (returns (Result :type Boolean))
  (return (`|EnumEquality` (`self.StateType`) "NewEnumerator1")))

(fn `Is State Idling`
  (returns (Result :type Boolean))
  (return (`|EnumEquality` (`self.StateType`) "NewEnumerator0")))

(fn `IsPlayer`
  (returns (Result :type Boolean))
  (return false))

(fn `Set Current Item`
  (params (`New Item` :type "/Game/Item/BP_Item Object Reference"))
  (returns (Result :type Boolean))
  (return false))

(fn `SetCanMove`
  (params (InCanMove :type Boolean))
  (returns (Result :type Boolean))
  (return false))

(fn `SetStateAction`
  (returns (Result :type Boolean))
  (set `self.StateType` "NewEnumerator1")
  (return false))

(fn `SetStateIdle`
  (returns (Result :type Boolean))
  (set `self.StateType` "NewEnumerator0")
  (return false))

(fn `UserConstructionScript`
  (`parent.UserConstructionScript`))