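; BP_Enemy is an enemy actor that shows a health bar and spawns damage number effects when hit.
; BeginPlay fills the WB_Health widget from StatusComponent.
; AnyDamage calls the parent handler, spawns BP_DamageEffect with the damage value at HitLocation, then reveals and refreshes the bar.
; SetLocation stores HitLocation with an upward offset, while DamageText and DeBuff are stubs returning false.
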(event `self.ReceiveBeginPlay`
  (bind _statuscomponent (`self.StatusComponent`))
  (bind _aswb_health (cast `/Game/Widgets/WB_Health` (`WidgetComponent.GetUserWidgetObject` (`self.HPBar`))))
  (`/Game/Widgets/WB_Health.UpdateHealthBar` _aswb_health (`/Game/Office/Component/StatusComponent.Health` _statuscomponent) (`/Game/Office/Component/StatusComponent.MaxHealth` _statuscomponent)))

(event `self.ReceiveAnyDamage`
  (params (Damage :type "Float (single-precision)") (DamageType :type "DamageType Object Reference") (InstigatedBy :type "Controller Object Reference") (DamageCauser :type "Actor Object Reference"))
  (bind _hpbar (`self.HPBar`))
  (bind _statuscomponent (`self.StatusComponent`))
  (`parent.ReceiveAnyDamage` Damage DamageType InstigatedBy DamageCauser)
  (bind _returnvalue (`|SpawnActorFromClass` "/Game/Widgets/BP_DamageEffect.BP_DamageEffect_C" (`KismetMathLibrary.Conv_VectorToTransform` (`self.HitLocation`)) "Undefined" "OverrideRootScale" null null))
  (`/Game/Widgets/BP_DamageEffect.SetDamageTExt` _returnvalue Damage (`self.HitLocation`))
  (`SceneComponent.SetVisibility` _hpbar true false)
  (bind _aswb_health (cast `/Game/Widgets/WB_Health` (`WidgetComponent.GetUserWidgetObject` _hpbar)))
  (`/Game/Widgets/WB_Health.UpdateHealthBar` _aswb_health (`/Game/Office/Component/StatusComponent.Health` _statuscomponent) (`/Game/Office/Component/StatusComponent.MaxHealth` _statuscomponent)))

(fn `DamageText`
  (params (Location :type "Vector Structure"))
  (returns (Result :type Boolean))
  (return false))

(fn `DeBuff`
  (params (DeBuff :type "/Game/Office/Enum/EEffect Enum" :default "NewEnumerator0") (Effect :type "/Game/Office/Enum/EEffect Enum" :default "NewEnumerator0") (Actor :type "/Game/GameCharacter/BP_DefaultCharacter Object Reference"))
  (returns (Result :type Boolean))
  (return false))

(fn `Set Location`
  (params (Lopcation :type "Vector Structure"))
  (set `self.HitLocation` (+ Lopcation (0.0 0.0 50.0))))

(fn `UserConstructionScript`)