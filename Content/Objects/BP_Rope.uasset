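; BP_Rope is a physics-driven rope actor that the player can grab and swing on.
; When a player overlaps its sphere, half their velocity becomes an impulse on CableEnd and the rope passes itself to the player via GrabRopeMessage.
; AddSwingingForce applies scaled force to CableEnd only while that end hangs less than a fixed vertical distance below the actor's origin.
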(event `self.Shpere.OnComponentBeginOverlap`
  (params (OverlappedComponent :type "PrimitiveComponent Object Reference") (OtherActor :type "Actor Object Reference") (OtherComp :type "PrimitiveComponent Object Reference") (OtherBodyIndex :type Integer) (bFromSweep :type Boolean) (SweepResult :type "HitResult Structure (by ref)"))
  (bind _result (message `/Game/Office/Interfaces/IState.IsPlayer` OtherActor))
  (if _result
    (`PrimitiveComponent.AddImpulse` (`self.CableEnd`) (* (`self.GetVelocity` OtherActor) 0.5) "None" false)
    (message `/Game/Office/Interfaces/IState.GrabRope` OtherActor self)))

(event `Add Swinging Force`
  (params (SwingForce :type "Vector Structure"))
  (bind (_returnvalue_x _returnvalue_y _returnvalue_z) (`KismetMathLibrary.BreakVector` (`self.K2_GetActorLocation`)))
  (bind (_returnvalue_x_2 _returnvalue_y_2 _returnvalue_z_2) (`KismetMathLibrary.BreakVector` (`SceneComponent.K2_GetComponentLocation` (`self.CableEnd`))))
  (if (< (- _returnvalue_z _returnvalue_z_2) 800.0)
    (`PrimitiveComponent.AddForce` (`self.CableEnd`) (* SwingForce 50000.0) "None" false)))

(fn `UserConstructionScript`)