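; BP_Weapon is a weapon base Blueprint that drives basic and tech attack combos from data tables.
; On BeginPlay it filters two data tables by WeaponType into separate combo arrays.
; The combo functions play the montage at the current count on the owning Character and set whether movement is allowed.
; EndAction returns to idle and resets combo state, while Attack and SendDamage are empty stubs.
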(event `self.ReceiveBeginPlay`
  ;[1 1 1] DT 받아오기
  (`parent.ReceiveBeginPlay`)
  (`|ExecutionSequence`
    (:`then_0`
      (bind _outrownames (`DataTableFunctionLibrary.GetDataTableRowNames` (`self.Data Table`)))
      (for _array_element _outrownames
        (bind _returnvalue (`|GetDataTableRow` (`self.Data Table`) _array_element)
          (:`then`
            (if (== (`.Type_2_2D806B9E4E19DA88DDF8EEA9EC46A9CE` (break `/Game/Office/Strcuts/FWeaponType` _returnvalue)) (`self.WeaponType`))
              (`KismetArrayLibrary.Array_Add` (`self.Weapon Datas`) _returnvalue))))))
    (:`then_1`
      (bind _outrownames_2 (`DataTableFunctionLibrary.GetDataTableRowNames` (`self.Tech_Data Table`)))
      (for _array_element_2 _outrownames_2
        (bind _returnvalue_2 (`|GetDataTableRow` (`self.Tech_Data Table`) _array_element_2)
          (:`then`
            (if (== (`.Type_2_2D806B9E4E19DA88DDF8EEA9EC46A9CE` (break `/Game/Office/Strcuts/FWeaponType` _returnvalue_2)) (`self.WeaponType`))
              (`KismetArrayLibrary.Array_Add` (`self.Weapon Datas_Tech`) _returnvalue_2))))))))

(event `self.EndAction`
  (`parent.EndAction`)
  (`self.SetStateIdle`)
  (`self.SetCanMove` true)
  (set `self.Success Combo` false)
  (set `self.last Basic Combo` false)
  (set `self.ComboCount` 0)
  (set `self.TechComboCount` 0))

(fn `Attack`)

(fn `PlayComboMontage`
  (returns (Montage :type "AnimMontage Object Reference"))
  (bind (_output_type _output_montage _output_playrate _output_startsection _output_canmove) (break `/Game/Office/Strcuts/FWeaponType` (`|GetArrayItem` (`self.Weapon Datas`) (`self.ComboCount`))))
  (bind _ascharacter (cast `Character` (`self.GetOwner`)))
  (`Character.PlayAnimMontage` _ascharacter _output_montage _output_playrate _output_startsection)
  (`self.SetCanMove` _output_canmove)
  (return _output_montage))

(fn `PlayTechComboMontage`
  (returns (Montage :type "AnimMontage Object Reference"))
  (bind (_output_type _output_montage _output_playrate _output_startsection _output_canmove) (break `/Game/Office/Strcuts/FWeaponType` (`|GetArrayItem` (`self.Weapon Datas_Tech`) (`self.TechComboCount`))))
  (bind _ascharacter (cast `Character` (`self.GetOwner`)))
  (`Character.PlayAnimMontage` _ascharacter _output_montage _output_playrate _output_startsection)
  (`self.SetCanMove` _output_canmove)
  (return _output_montage))

(fn `SendDamage`)

(fn `UserConstructionScript`
  (`parent.UserConstructionScript`))