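; BP_HealthPotion is a consumable item that restores health to the player who owns it.
; On UseAction it casts its owner to BP_Player and adds a fixed amount directly to the StatusComponent's Health, with no clamp in this graph.
; The potion then destroys itself; if the owner is not a BP_Player, nothing happens.
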(event `self.ReceiveBeginPlay`
  (`parent.ReceiveBeginPlay`))

(event `/Game/Office/Interfaces/IAction.UseAction`
  (bind _asbp_player (cast `/Game/GameCharacter/Player/BP_Player` (`self.GetOwner`)))
  (bind _statuscomponent (`/Game/GameCharacter/BP_DefaultCharacter.StatusComponent` _asbp_player))
  (set `/Game/Office/Component/StatusComponent.Health` (+ (`/Game/Office/Component/StatusComponent.Health` _statuscomponent) 50.0) _statuscomponent)
  (`self.K2_DestroyActor`))

(fn `UserConstructionScript`
  (`parent.UserConstructionScript`))