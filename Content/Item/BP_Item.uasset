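; Base item Blueprint that defines input-action hooks for items and links them to their owner's state.
; Click, side-button combination and EndAction functions are empty stubs, apparently for child items to override.
; Helpers reach the owner through IState and IEquipItemType interface messages to read equip type, change state or toggle movement.
; CanAction passes only when the owner is idle, while IsStateAction discards the owner's answer and returns false.
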(fn `All Click`)

(fn `Can Action`
  (returns (ReturnValue :type Boolean))
  (return (`self.Is State Ideling`)))

(fn `EndAction`)

(fn `Get Item Type`
  (returns (`Equip Item` :type "/Game/Office/Enum/EItemType Enum"))
  (bind _returnvalue (`self.GetOwner`))
  (if (`KismetSystemLibrary.DoesImplementInterface` _returnvalue "/Game/Office/Interfaces/IEquipItemType.IEquipItemType_C")
    (bind _equip_item (message `/Game/Office/Interfaces/IEquipItemType.Get Equip Item` _returnvalue))
    (return _equip_item)))

(fn `Is State Action`
  (returns (Result :type Boolean))
  (bind _returnvalue (`self.GetOwner`))
  (if (`KismetSystemLibrary.DoesImplementInterface` _returnvalue "/Game/Office/Interfaces/IState.IState_C")
    (message `/Game/Office/Interfaces/IState.Is State Action` _returnvalue)
    (return false)))

(fn `Is State Ideling`
  (returns (Result :type Boolean))
  (bind _returnvalue (`self.GetOwner`))
  (if (`KismetSystemLibrary.DoesImplementInterface` _returnvalue "/Game/Office/Interfaces/IState.IState_C")
    (bind _result (message `/Game/Office/Interfaces/IState.Is State Idling` _returnvalue))
    (return _result)))

(fn `Left Click`)

(fn `Right Click`)

(fn `SetCanMove`
  (params (InCanMove :type Boolean))
  (bind _returnvalue (`self.GetOwner`))
  (if (`KismetSystemLibrary.DoesImplementInterface` _returnvalue "/Game/Office/Interfaces/IState.IState_C")
    (message `/Game/Office/Interfaces/IState.SetCanMove` _returnvalue (`local.InCanMove`))
    (return)))

(fn `SetStateAction`
  (bind _returnvalue (`self.GetOwner`))
  (if (`KismetSystemLibrary.DoesImplementInterface` _returnvalue "/Game/Office/Interfaces/IState.IState_C")
    (message `/Game/Office/Interfaces/IState.SetStateAction` _returnvalue)
    (return)))

(fn `SetStateIdle`
  (bind _returnvalue (`self.GetOwner`))
  (if (`KismetSystemLibrary.DoesImplementInterface` _returnvalue "/Game/Office/Interfaces/IState.IState_C")
    (message `/Game/Office/Interfaces/IState.SetStateIdle` _returnvalue)
    (return)))

(fn `Side And  Right Click`)

(fn `Side And Left Click`)

(fn `Side And SpaceBar`)

(fn `Side Click`)

(fn `UserConstructionScript`)