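; Sword equipment Blueprint, derived from a parent weapon class, that turns click and side-input combinations into basic, tech and quickdraw attacks.
; Input events set combo indices and play montages, or flag success during the CanCombo window so PlayNextCombo can advance the chain.
; QuickdrawReady diverts left and side clicks to quickdraw montages.
; Collision events toggle the Capsule, whose overlaps send DamageComponent's combo or tech damage to other BP_DefaultCharacters.
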(event `self.ReceiveBeginPlay`
  (`parent.ReceiveBeginPlay`)
  (`self.SetWeaponInfo`)
  (`PrimitiveComponent.SetCollisionEnabled` (`self.Capsule`) "NoCollision"))

(event `self.Side And SpaceBar`
  (`parent.Side And SpaceBar`)
  (if (`self.CanCombo`)
    (set `self.CanCombo` false)
    (set `self.Success Combo` true)
    (set `self.TechComboCount` 4)
    (`self.PlayTechComboMontage`)))

(event `self.Left Click`
  ;[1 1 1] 좌클릭(기본공격, 콤보)
  (`parent.Left Click`)
  (if (`self.QuickdrawReady`)
    (`self.Quickdraw1`)
    (elif (`self.CanCombo`)
      (if (`self.last Basic Combo`)
        (set `self.last Basic Combo` false)
        (set `self.ComboCount` 0)
        (set `self.CanCombo` false)
        (set `self.Success Combo` true)
        (else
          (set `self.CanCombo` false)
          (set `self.Success Combo` true)))
      (elif (`self.Can Action`)
        (`self.SetStateAction`)
        (`self.PlayComboMontage`)))))

(event `self.Side And  Right Click`
  (`parent.Side And  Right Click`)
  (if (`self.CanCombo`)
    (set `self.CanCombo` false)
    (set `self.Success Combo` true)
    (set `self.TechComboCount` 5)
    (`self.PlayTechComboMontage`)
    (elif (`self.Can Action`)
      (`self.SetStateAction`)
      (set `self.TechComboCount` 5)
      (`self.PlayTechComboMontage`))))

(event `Quickdraw1`
  (bind _ascharacter (cast `Character` (`self.GetOwner`)))
  (`Character.PlayAnimMontage` _ascharacter "/Game/Character/Montages/YinSword/Tech/Tach4.Tach4" 1.0 "None")
  (set `self.QuickdrawReady` false))

(event `self.Right Click`
  ;[1 1 1] 우클릭(기본공격, 콤보)
  (`parent.Right Click`)
  (if (`self.CanCombo`)
    (if (== (`self.ComboCount`) 2)
      (set `self.ComboCount` 0)
      (else
        (set `self.CanCombo` false)
        (set `self.Success Combo` true)
        (set `self.ComboCount` 1)))
    (elif (`self.Can Action`)
      (`self.SetStateAction`)
      (set `self.ComboCount` 2)
      (`self.PlayComboMontage`))))

(event `self.Side And Left Click`
  (`parent.Side And Left Click`)
  (if (`self.CanCombo`)
    (set `self.CanCombo` false)
    (set `self.Success Combo` true)
    (set `self.TechComboCount` 6)
    (`self.PlayTechComboMontage`)
    (elif (`self.Can Action`)
      (`self.SetStateAction`)
      (set `self.TechComboCount` 6)
      (`self.PlayTechComboMontage`))))

(event `Quickdraw2`
  (bind _ascharacter (cast `Character` (`self.GetOwner`)))
  (`Character.PlayAnimMontage` _ascharacter "/Game/Character/Montages/YinSword/Tech/QuickDraw1.QuickDraw1" 1.0 "None")
  (set `self.QuickdrawReady` false))

(event `self.All Click`
  ;[1 1 1] 양쪽 클릭 (특수 공격, 콤보)
  (`parent.All Click`)
  (if (`self.CanCombo`)
    (set `self.CanCombo` false)
    (set `self.Success Combo` true)
    (set `self.ComboCount` 4)
    (`self.PlayComboMontage`)
    (elif (`self.Can Action`)
      (`self.SetStateAction`)
      (set `self.ComboCount` 4)
      (`self.PlayComboMontage`))))

(event `self.Side Click`
  ;[1 1 1] 특수 공격
  (`parent.Side Click`)
  (if (`self.QuickdrawReady`)
    (`self.Quickdraw2`)
    (elif (`self.Basic Attack`)
      (set `self.Basic Attack` false)
      (set `self.CanCombo` false)
      (`self.SetStateAction` :!label _label)
      (`self.PlayTechComboMontage`)
      (elif (`self.CanCombo`)
        (set `self.CanCombo` false)
        (set `self.Success Combo` true)
        (set `self.Tech` true)
        (elif (`self.Can Action`)
          (goto _label))))))

(event `PlayNextCombo`
  (if (`self.Success Combo`)
    (`self.SetStateAction`)
    (set `self.Success Combo` false)
    (if (`self.Tech`)
      (set `self.Tech` false)
      (bind _result (`/Engine/EditorBlueprintResources/StandardMacros.IncrementInt` (`self.TechComboCount`))
        (:`  `
          (`self.PlayTechComboMontage`)
          (if (== _result 3)
            _)))
      (else
        (bind _result_2 (`/Engine/EditorBlueprintResources/StandardMacros.IncrementInt` (`self.ComboCount`))
          (:`  `
            (`self.PlayComboMontage`)
            (if (== _result_2 3)
              (set `self.last Basic Combo` true)
              (else
                (set `self.last Basic Combo` false)))))))))

(event `self.Capsule.OnComponentBeginOverlap`
  (params (OverlappedComponent :type "PrimitiveComponent Object Reference") (OtherActor :type "Actor Object Reference") (OtherComp :type "PrimitiveComponent Object Reference") (OtherBodyIndex :type Integer) (bFromSweep :type Boolean) (SweepResult :type "HitResult Structure (by ref)"))
  (if (!= OtherActor (`self.GetOwner`))
    (bind _asbp_default_character (cast `/Game/GameCharacter/BP_DefaultCharacter` OtherActor))
    (if (`self.Tech`)
      (bind (_damage _tech_damage_type) (`/Game/Office/Component/DamageComponent.Get TechDamage` (`self.DamageComponent`) (`self.TechComboCount`)))
      (`self.SendDamage` _asbp_default_character _damage _tech_damage_type)
      (else
        (bind (_damage_2 _damage_type) (`/Game/Office/Component/DamageComponent.Get Damage` (`self.DamageComponent`) (`self.ComboCount`)))
        (`self.SendDamage` _asbp_default_character _damage_2 _damage_type)))))

(event `self.OnCollision`
  (`parent.OnCollision`)
  (`PrimitiveComponent.SetCollisionEnabled` (`self.Capsule`) "QueryOnly"))

(event `self.OffCollision`
  (`parent.OffCollision`)
  (`PrimitiveComponent.SetCollisionEnabled` (`self.Capsule`) "NoCollision"))

(fn `UserConstructionScript`)