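; BP_Weapon is an equippable weapon, with empty Attack, Awakening and OnCollision functions.
; BeginPlay filters three DataTables by WeaponType into basic combo, tech combo and stat arrays, which feed montage playback, movement locking and DamageComponent stat setup.
; SendDamage uses a hit-actor list, cleared by OffCollision, to avoid repeat damage to characters.
; UseAction pushes item info to the player's HUD, and EndAction resets combo and movement state.
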(event `self.ReceiveBeginPlay`
  ;[1 1 1] DT 받아오기
  (`parent.ReceiveBeginPlay`)
  (`|ExecutionSequence`
    (:`then_0`
      (bind _outrownames (`DataTableFunctionLibrary.GetDataTableRowNames` (`self.Data Table`)))
      (for _array_element _outrownames
        (bind _returnvalue (`|GetDataTableRow` (`self.Data Table`) _array_element)
          (:`then`
            (if (== (`.Type_2_2D806B9E4E19DA88DDF8EEA9EC46A9CE` (break `/Game/Office/Strcuts/FWeaponType` _returnvalue)) (`self.WeaponType`))
              (`KismetArrayLibrary.Array_Add` (`self.Weapon Datas`) _returnvalue))))))
    (:`then_1`
      (bind _outrownames_2 (`DataTableFunctionLibrary.GetDataTableRowNames` (`self.Tech_Data Table`)))
      (for _array_element_2 _outrownames_2
        (bind _returnvalue_2 (`|GetDataTableRow` (`self.Tech_Data Table`) _array_element_2)
          (:`then`
            (if (== (`.Type_2_2D806B9E4E19DA88DDF8EEA9EC46A9CE` (break `/Game/Office/Strcuts/FWeaponType` _returnvalue_2)) (`self.WeaponType`))
              (`KismetArrayLibrary.Array_Add` (`self.Weapon Datas_Tech`) _returnvalue_2))))))
    (:`then_2`
      (bind _outrownames_3 (`DataTableFunctionLibrary.GetDataTableRowNames` (`self.InfoDataTable`)))
      (for _array_element_3 _outrownames_3
        (bind _returnvalue_3 (`|GetDataTableRow` (`self.InfoDataTable`) _array_element_3)
          (:`then`
            (if (`|EnumEquality` (`.WeaponType_4_B911139F43865B99B730CDAF594278E8` (break `/Game/Office/Strcuts/FWeaponinfo` _returnvalue_3)) (`self.WeaponType`))
              (`KismetArrayLibrary.Array_Add` (`self.WeaponInfoDatas`) _returnvalue_3))))))))

(event `self.EndAction`
  (`parent.EndAction`)
  (`self.SetStateIdle`)
  (`self.SetCanMove` true)
  (set `self.Success Combo` false)
  (set `self.last Basic Combo` false)
  (set `self.ComboCount` 0)
  (set `self.TechComboCount` 0)
  (set `self.Tech` false))

(event `/Game/Office/Interfaces/IAction.UseAction`
  (bind _equipinfo (`self.EquipInfo`))
  (bind (_item _itemimage) (break `/Game/Office/Strcuts/FInventory` (`self.ItemInfo`)))
  (bind _asbp_player (cast `/Game/GameCharacter/Player/BP_Player` (`self.GetOwner`)))
  (setmembers `/Game/Office/Strcuts/FCharInfo` :`StructRef` _equipinfo :`Item` _item :`ItemImage` _itemimage)
  (bind _gamehud (`/Game/GameCharacter/Player/BP_Player.GameHUD` _asbp_player))
  (bind _playerweapon (`/Game/Widgets/WB_PlayerHUD.PlayerWeapon` _gamehud))
  (set `/Game/Widgets/WB_PlayerInventory.ItemImage` _itemimage _playerweapon)
  (set `/Game/Widgets/WB_PlayerInventory.Item` _item _playerweapon)
  (`KismetArrayLibrary.Array_Add` (`/Game/Widgets/WB_PlayerHUD.CharInfo` _gamehud) _equipinfo)
  (`/Game/Widgets/WB_PlayerHUD.EquipInfo` _gamehud))

(fn `Attack`)

(fn `Awakening`)

(fn `GetOwnerInfo`
  (cast `Character` (`self.GetOwner`)))

(fn `OffCollision`
  (`KismetArrayLibrary.Array_Clear` (`self.HittedActors`)))

(fn `OnCollision`)

(fn `PlayComboMontage`
  (returns (Montage :type "AnimMontage Object Reference") (MonatgeTime :type "Float (double-precision)"))
  (bind (_output_type _output_montage _output_playrate _output_startsection _output_canmove) (break `/Game/Office/Strcuts/FWeaponType` (`|GetArrayItem` (`self.Weapon Datas`) (`self.ComboCount`))))
  (bind _asbp_default_character (cast `/Game/GameCharacter/BP_DefaultCharacter` (`self.GetOwner`)))
  (bind _returnvalue (`AnimInstance.Montage_Play` (`SkeletalMeshComponent.GetAnimInstance` (`Character.Mesh` _asbp_default_character)) _output_montage _output_playrate "MontageLength" 0.0 true))
  (`self.SetCanMove` _output_canmove)
  (return _output_montage _returnvalue))

(fn `PlayTechComboMontage`
  (returns (Montage :type "AnimMontage Object Reference") (ReturnValue :type "Float (double-precision)"))
  (bind (_output_type _output_montage _output_playrate _output_startsection _output_canmove) (break `/Game/Office/Strcuts/FWeaponType` (`|GetArrayItem` (`self.Weapon Datas_Tech`) (`self.TechComboCount`))))
  (bind _asbp_default_character (cast `/Game/GameCharacter/BP_DefaultCharacter` (`self.GetOwner`)))
  (bind _returnvalue (`AnimInstance.Montage_Play` (`SkeletalMeshComponent.GetAnimInstance` (`Character.Mesh` _asbp_default_character)) _output_montage _output_playrate "MontageLength" 0.0 true))
  (`self.SetCanMove` _output_canmove)
  (return _output_montage _returnvalue))

(fn `SendDamage`
  (params (`Other Actor` :type "Actor Object Reference") (Damage :type "Float (double-precision)") (DamageType :type "DamageType Class Reference"))
  (returns (result :type Boolean))
  (locals (EverHittedActor :type Boolean))
  (for _array_element (`self.HittedActors`)
    (if (== _array_element (`local.Other Actor`))
      (set `local.EverHittedActor` true)
      (break)))
  (if (not (`local.EverHittedActor`))
    (`KismetArrayLibrary.Array_Add` (`self.HittedActors`) (`local.Other Actor`))
    (if (!= `Other Actor` (`self.GetOwner`))
      (bind _ascharacter (cast `Character` (`local.Other Actor`)))
      (`GameplayStatics.ApplyDamage` _ascharacter (`local.Damage`) (`self.GetInstigatorController` (`self.GetOwner`)) self DamageType)
      (return false))))

(fn `SetWeaponInfo`
  (returns (AttackPower :type "Float (double-precision)") (AttackSpeed :type "Float (double-precision)") (Critical :type "Float (double-precision)"))
  (bind (_output_weapontype _output_attackpower _output_attackspeed _output_critical) (break `/Game/Office/Strcuts/FWeaponinfo` (`|GetArrayItem` (`self.WeaponInfoDatas`))))
  (bind (_attackpower _attackspeed _critical) (`/Game/Office/Component/DamageComponent.GetWeaponInfo` (`self.DamageComponent`) _output_attackpower _output_attackspeed _output_critical))
  (return _attackpower _attackspeed _critical))

(fn `UserConstructionScript`
  (`parent.UserConstructionScript`))