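; Boss melee weapon that plays randomized combo montages for left, right, upper and multi-hit attacks.
; Each attack picks ComboCount from its own index range; ComboAttack chooses the range by the sign of Dot.
; Left and right attacks repeat recursively after montage-length delays, while ComboAttack uses a delayed-loop macro.
; Sphere overlaps with non-owner BP_Enemy actors send damage that DamageComponent looks up by ComboCount.
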(event `LeftAttack`
  (params (Playcount :type Integer))
  (if (`self.Can Action`)
    (`self.SetStateAction`)
    (set `self.ComboCount` (`KismetMathLibrary.RandomIntegerInRange` 0 2))
    (bind (_montage _monatgetime) (`self.PlayComboMontage`))
    (`KismetSystemLibrary.Delay` _monatgetime)
    (if (== Playcount 0)
      (`Controller.StopMovement` (`self.GetInstigatorController`))
      (else
        (bind _result (`/Engine/EditorBlueprintResources/StandardMacros.DecrementInt` Playcount)
          (:`  `
            (if (== _result 0)
              (`self.LeftAttack` 0)
              (else
                (`self.LeftAttack` _result)))))))))

(event `RightAttack`
  (params (Playcount2 :type Integer))
  (if (`self.Can Action`)
    (`self.SetStateAction`)
    (set `self.ComboCount` (+ (`KismetMathLibrary.RandomIntegerInRange` 0 2) 3))
    (bind (_montage _monatgetime) (`self.PlayComboMontage`))
    (`KismetSystemLibrary.Delay` _monatgetime)
    (if (== Playcount2 0)
      (`Controller.StopMovement` (`self.GetInstigatorController`))
      (else
        (bind _result (`/Engine/EditorBlueprintResources/StandardMacros.DecrementInt` Playcount2)
          (:`  `
            (if (== _result 0)
              (`self.RightAttack` 0)
              (else
                (`self.RightAttack` _result)))))))))

(event `ComboAttack`
  (params (ComboAttackCount :type Integer) (Dot :type "Float (double-precision)") (NewParam :type Boolean))
  (`self.ForLoopDelay` 0 ComboAttackCount (stale _monatgetime)
    (:`LoopBody`
      (set `self.ComboCount` (`KismetMathLibrary.RandomIntegerInRange` 0 2))
      (if (not (>= 0.0 Dot))
        (set `self.ComboCount` (+ (`self.ComboCount`) 3)))
      (if (`self.Can Action`)
        (`self.SetStateAction`)
        (bind (_montage _monatgetime) (`self.PlayComboMontage`))))))

(event `UpperAttack`
  (set `self.ComboCount` (`KismetMathLibrary.RandomIntegerInRange` 7 8))
  (`self.SetStateAction`)
  (`self.PlayComboMontage`))

(event `self.Sphere.OnComponentBeginOverlap`
  (params (OverlappedComponent :type "PrimitiveComponent Object Reference") (OtherActor :type "Actor Object Reference") (OtherComp :type "PrimitiveComponent Object Reference") (OtherBodyIndex :type Integer) (bFromSweep :type Boolean) (SweepResult :type "HitResult Structure (by ref)"))
  (if (!= OtherActor (`self.GetOwner`))
    (bind _asbp_enemy (cast `/Game/GameCharacter/Enemies/EnemyAI/BP_Enemy` OtherActor))
    (bind _damage (`/Game/Office/Component/DamageComponent.Get Damage` (`self.DamageComponent`) (`self.ComboCount`)))
    (`self.SendDamage` _asbp_enemy _damage)))

(fn `MeleeAttack`)

(fn `UserConstructionScript`
  (`parent.UserConstructionScript`))