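; BP_EffcetBurning is a short-lived burning status effect that deals damage over time to the character it is attached to.
; On BeginPlay it sets a lifespan just under three seconds and starts a looping one-second timer, so damage lands twice.
; Each tick casts the attach parent to BP_DefaultCharacter, applies a tenth of its StatusComponent MaxHealth with the instigator as damage causer, and prints the result.
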(event `self.ReceiveBeginPlay`
  (`self.SetLifeSpan` 2.9)
  (`KismetSystemLibrary.K2_SetTimerDelegate` (delegate `Burning`) 1.0 true))

(event `Burning`
  (bind _returnvalue (`self.GetAttachParentActor`))
  (bind _asbp_default_character (cast `/Game/GameCharacter/BP_DefaultCharacter` _returnvalue))
  (bind _returnvalue_2 (`GameplayStatics.ApplyDamage` _returnvalue (* (`/Game/Office/Component/StatusComponent.MaxHealth` (`/Game/GameCharacter/BP_DefaultCharacter.StatusComponent` _asbp_default_character)) 0.1) null (`self.GetInstigator`)))
  (`KismetSystemLibrary.PrintString` (`KismetStringLibrary.Conv_DoubleToString` _returnvalue_2)))

(fn `UserConstructionScript`)