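; Player character with camera-relative movement, montage-driven sword equip, a cable grappling hook, potion selection and a ragdoll key.
; BeginPlay spawns sword and dual dagger, creates the potion widget and fills the potion list cycled by mouse wheel.
; Clicks and jump enter a short input buffer that detects two-button chords, forwarding single or combined clicks to the equipped item.
; Grappling line-traces forward, then Tick applies steerable force toward the hit point in flying mode.
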(event `Key|X`
  (params (Key :type "Key Structure"))
  (bind _mesh (`self.Mesh`))
  (:`Pressed`
    (`PrimitiveComponent.SetSimulatePhysics` (`self.Mesh`) true)
    (`PrimitiveComponent.SetCollisionEnabled` _mesh "QueryAndPhysics")
    (`PrimitiveComponent.AddForce` _mesh (0.0 0.0 0.0) "None" false)))

(event `InputAxis|MoveForward`
  (params (AxisValue :type "Float (single-precision)"))
  (bind (_returnvalue_roll _returnvalue_pitch _returnvalue_yaw) (`KismetMathLibrary.BreakRotator` (`self.GetControlRotation`)))
  (if (`self.CanMove`)
    (`self.AddMovementInput` (`KismetMathLibrary.GetForwardVector` (`KismetMathLibrary.MakeRotator` 0.0 0.0 _returnvalue_yaw)) AxisValue)))

(event `InputAxis|MoveRight`
  (params (AxisValue :type "Float (single-precision)"))
  (bind (_returnvalue_roll _returnvalue_pitch _returnvalue_yaw) (`KismetMathLibrary.BreakRotator` (`self.GetControlRotation`)))
  (if (`self.CanMove`)
    (`self.AddMovementInput` (`KismetMathLibrary.GetRightVector` (`KismetMathLibrary.MakeRotator` 0.0 0.0 _returnvalue_yaw)) AxisValue)))

(event `InputAction|Walking`
  (params (Key :type "Key Structure"))
  (bind _charactermovement (`self.CharacterMovement`))
  (:`Pressed`
    (set `CharacterMovementComponent.MaxWalkSpeed` 400.0 _charactermovement))
  (:`Released`
    (set `CharacterMovementComponent.MaxWalkSpeed` 600.0 _charactermovement)))

(event `InputAction|LeftClick`
  (params (Key :type "Key Structure"))
  (:`Pressed`
    (`KismetArrayLibrary.Array_Add` (`self.Click`) Key)
    (`KismetSystemLibrary.Delay` 0.1)
    (bind _returnvalue (`self.Is Special Key`))
    (if _returnvalue
      (bind _equip_current_item (`self.Equip Current Item`)
        (:`then`
          (`/Game/Item/BP_Item.Left Click` _equip_current_item))
        (:`else`))
      (else
        (`self.SpecialKey`)))))

(event `InputAction|RightClick`
  (params (Key :type "Key Structure"))
  (:`Pressed`
    (`KismetArrayLibrary.Array_Add` (`self.Click`) Key)
    (`KismetSystemLibrary.Delay` 0.1)
    (bind _returnvalue (`self.Is Special Key`))
    (if _returnvalue
      (bind _equip_current_item (`self.Equip Current Item`)
        (:`then`
          (`/Game/Item/BP_Item.Right Click` _equip_current_item))
        (:`else`))
      (else
        (`self.SpecialKey`)))))

(event `InputAction|SideMouse`
  (params (Key :type "Key Structure"))
  (:`Pressed`
    (`KismetArrayLibrary.Array_Add` (`self.Click`) Key)
    (`KismetSystemLibrary.Delay` 0.1)
    (bind _returnvalue (`self.Is Special Key`))
    (if _returnvalue
      (bind _equip_current_item (`self.Equip Current Item`)
        (:`then`
          (`/Game/Item/BP_Item.Side Click` _equip_current_item))
        (:`else`))
      (else
        (`self.SpecialKey`)))))

(event `InputAction|Jumping`
  (params (Key :type "Key Structure"))
  (:`Pressed`
    (`KismetArrayLibrary.Array_Add` (`self.Click`) Key)
    (`KismetSystemLibrary.Delay` 0.1)
    (`|ExecutionSequence`
      (:`then_0`
        (bind _returnvalue (`self.Is Special Key`))
        (if (not _returnvalue)
          (`self.SpecialKey`)))
      (:`then_1`
        (if (`self.CanMove`)
          (`self.Jump`))))))

(event `SpecialKey`
  (switch `/Game/Office/Enum/EClickType` (`self.ClickType`)
    (:`NewEnumerator2`
      (bind _equip_current_item (`self.Equip Current Item`)
        (:`then`
          (`/Game/Item/BP_Item.All Click` _equip_current_item))
        (:`else`)))
    (:`NewEnumerator4`
      (bind _equip_current_item_2 (`self.Equip Current Item`)
        (:`then`
          (`/Game/Item/BP_Item.Side And Left Click` _equip_current_item_2))
        (:`else`)))
    (:`NewEnumerator5`
      (bind _equip_current_item_3 (`self.Equip Current Item`)
        (:`then`
          (`/Game/Item/BP_Item.Side And  Right Click` _equip_current_item_3))
        (:`else`)))
    (:`NewEnumerator6`
      (bind _equip_current_item_4 (`self.Equip Current Item`)
        (:`then`
          (`/Game/Item/BP_Item.Side And SpaceBar` _equip_current_item_4))
        (:`else`))))
  (set `self.ClickType` "NewEnumerator7"))

(event `InputAxis|HorizontalLook`
  (params (AxisValue :type "Float (single-precision)"))
  (`self.AddControllerYawInput` AxisValue))

(event `InputAxis|VerticalLook`
  (params (AxisValue :type "Float (single-precision)"))
  (`self.AddControllerPitchInput` AxisValue))

(event `self.ReceiveBeginPlay`
  (bind _potion (`self.Potion`))
  (`|ExecutionSequence`
    (:`then_0`
      (bind _returnvalue (`|SpawnActorFromClass` "/Game/Item/Weapon/BP_Sword.BP_Sword_C" (`KismetMathLibrary.MakeTransform` (0.0 0.0 0.0)) "Undefined" "OverrideRootScale" self null))
      (bind _output_get (set `self.Sowrd` _returnvalue))
      (`self.K2_AttachToComponent` _output_get (`self.Mesh`) "Holster_Sword" "KeepRelative" "KeepRelative" "KeepRelative" true)
      (`SkinnedMeshComponent.HideBoneByName` (`self.Mesh`) "weapon_r" "PBO_None"))
    (:`then_1`
      (bind _returnvalue_2 (`|SpawnActorFromClass` "/Game/Item/Weapon/BP_DualSword.BP_DualSword_C" (`KismetMathLibrary.MakeTransform` (0.0 0.0 0.0)) "Undefined" "OverrideRootScale" self null))
      (set `self.Dual Dagger` _returnvalue_2))
    (:`then_2`
      (bind _returnvalue_3 (`|CreateWidget` "/Game/Widgets/WB_PotionContainer.WB_PotionContainer_C" (`GameplayStatics.GetPlayerController` 0)))
      (bind _output_get_2 (set `self.PotionWidget` _returnvalue_3))
      (`UserWidget.AddToViewport` _output_get_2 0))
    (:`then_3`
      (`|ExecutionSequence`
        (:`then_0`
          (`KismetArrayLibrary.Array_Add` (`self.PotionSelect`) (make `/Game/Office/Strcuts/FPotionType` (`/Game/Item/Utile/BP_ConsumptionItem.HealthPotion` _potion))))
        (:`then_1`
          (`KismetArrayLibrary.Array_Add` (`self.PotionSelect`) (make `/Game/Office/Strcuts/FPotionType` (`/Game/Item/Utile/BP_ConsumptionItem.BurnPotion` _potion))))
        (:`then_2`
          (`KismetArrayLibrary.Array_Add` (`self.PotionSelect`) (make `/Game/Office/Strcuts/FPotionType` (`/Game/Item/Utile/BP_ConsumptionItem.FrostbitePotion` _potion))))))))

(event `InputAction|Sword`
  (params (Key :type "Key Structure"))
  (:`Pressed`
    (if (`|EnumEquality` (`self.Weapon Type`) "NewEnumerator0")
      (`self.UnequipSword`)
      (else
        (`self.EquipSword`)))))

(event `EquippedSword`
  (set `self.CanMove` true)
  (set `self.StateType` "NewEnumerator0")
  (set `self.bUseControllerRotationYaw` true)
  (set `CharacterMovementComponent.bOrientRotationToMovement` false (`self.CharacterMovement`))
  (set `self.Weapon Type` "NewEnumerator0")
  (set `self.Item Type` "NewEnumerator1")
  (`self.Set Current Item` (`self.Sowrd`)))

(event `EquipSword`
  (set `self.StateType` "NewEnumerator2")
  (`self.PlayAnimMontage` "/Game/Character/Montages/YinSword/Yin_Sword_Equip.Yin_Sword_Equip"))

(event `UnequipSword`
  (set `self.StateType` "NewEnumerator3")
  (`self.PlayAnimMontage` "/Game/Character/Montages/YinSword/Yin_Sword_UnEquip.Yin_Sword_UnEquip"))

(event `UnequippedSword`
  (set `self.CanMove` true)
  (set `self.StateType` "NewEnumerator0")
  (set `self.bUseControllerRotationYaw` false)
  (set `CharacterMovementComponent.bOrientRotationToMovement` true (`self.CharacterMovement`))
  (set `self.Weapon Type` "NewEnumerator2")
  (set `self.Item Type` "NewEnumerator0"))

(event `AttachSword`
  (`self.K2_AttachToComponent` (`self.Sowrd`) (`self.Mesh`) "Hand_Sword" "KeepRelative" "KeepRelative" "KeepRelative" true))

(event `DetachSword`
  (`self.K2_AttachToComponent` (`self.Sowrd`) (`self.Mesh`) "Holster_Sword" "KeepRelative" "KeepRelative" "KeepRelative" true))

(event `self.ReceiveTick`
  (params (DeltaSeconds :type "Float (single-precision)"))
  (`|ExecutionSequence`
    (:`then_0`
      (if (`self.Is Grappling`)
        (set `CableComponent.EndLocation` (`KismetMathLibrary.InverseTransformLocation` (`self.GetTransform`) (`self.Grab Point`)) (`self.Cable`))
        (`CharacterMovementComponent.AddForce` (`self.CharacterMovement`) (* (`KismetMathLibrary.Normal` (+ (`KismetMathLibrary.GetDirectionUnitVector` (`self.K2_GetActorLocation`) (`self.Grab Point`)) (* (* (`self.GetActorRightVector`) (`self.GetInputAxisValue`)) 0.7))) 250000.0))))
    (:`then_1`
      (`KismetSystemLibrary.PrintString` (`|GetEnumeratorNameAsString` (`self.StateType`)) true true (struct :`G` 0.66 :`B` 1.0 :`A` 1.0) (`GameplayStatics.GetWorldDeltaSeconds`)))))

(event `Key|C`
  (params (Key :type "Key Structure"))
  (bind _returnvalue (`self.K2_GetActorLocation`))
  (:`Pressed`
    (bind (_outhit _returnvalue_2) (`KismetSystemLibrary.LineTraceSingle` _returnvalue (+ _returnvalue (* (`KismetMathLibrary.GetForwardVector` (`self.K2_GetActorRotation` (`GameplayStatics.GetPlayerController` 0))) 3000.0)) "TraceTypeQuery1"))
    (if _returnvalue_2
      (set `self.Grab Point` (`.ImpactPoint` (`GameplayStatics.BreakHitResult` _outhit)))
      (set `self.Is Grappling` true)
      (`CharacterMovementComponent.SetMovementMode` (`self.CharacterMovement`) "MOVE_Flying" 0)
      (`SceneComponent.SetHiddenInGame` (`self.Cable`) false false)))
  (:`Released`
    (set `self.Is Grappling` false)
    (`CharacterMovementComponent.SetMovementMode` (`self.CharacterMovement`) "MOVE_Falling" 0)
    (`SceneComponent.SetHiddenInGame` (`self.Cable`) true false)))

(event `InputAction|WheelUp`
  (params (Key :type "Key Structure"))
  (:`Pressed`
    (bind _result (`/Engine/EditorBlueprintResources/StandardMacros.IncrementInt` (`self.PotionIndex`))
      (:`  `
        (set `self.PotionIndex` (mod _result (`KismetArrayLibrary.Array_Length` (`self.PotionSelect`))))))))

(event `InputAction|WheelDown`
  (params (Key :type "Key Structure"))
  (:`Pressed`
    (bind _result (`/Engine/EditorBlueprintResources/StandardMacros.DecrementInt` (`self.PotionIndex`))
      (:`  `
        (if (< _result 0)
          (set `self.PotionIndex` (- (`KismetArrayLibrary.Array_Length` (`self.PotionSelect`)) 1)))))))

(event `self.Sword.OnComponentBeginOverlap`
  (params (OverlappedComponent :type "PrimitiveComponent Object Reference") (OtherActor :type "Actor Object Reference") (OtherComp :type "PrimitiveComponent Object Reference") (OtherBodyIndex :type Integer) (bFromSweep :type Boolean) (SweepResult :type "HitResult Structure (by ref)"))
  (if (!= OtherActor self)
    (bind _asbp_enemy (cast `/Game/Enemies/BP_Enemy` OtherActor))
    (`/Game/Enemies/BP_Enemy.MakeRagdoll` _asbp_enemy)))

(fn `DeQueue`
  (`KismetArrayLibrary.Array_Clear` (`self.Click`)))

(fn `Get Current Item`
  (returns (`Current Item` :type "/Game/Item/BP_Item Object Reference"))
  (return (`self.Equip Current Item`)))

(fn `Get Equip Item`
  (returns (`Equip Item` :type "/Game/Office/Enum/EItemType Enum"))
  (return (`self.Item Type`)))

(fn `Get Side and Left`
  (returns (ReturnValue :type Boolean))
  (return (and (`self.Side Click`) (`self.Left Click`))))

(fn `Get Side and Right`
  (returns (ReturnValue :type Boolean))
  (return (and (`self.Side Click`) (`self.Right Click`))))

(fn `Get Side and Space`
  (returns (ReturnValue :type Boolean))
  (return (and (`self.Side Click`) (`self.SpaceBar Click`))))

(fn `Get Two All Click`
  (returns (ReturnValue :type Boolean))
  (return (and (`self.Left Click`) (`self.Right Click`))))

(fn `InputQueue`
  (bind _click (`self.Click`))
  (bind _click_2 (`self.Click`))
  (bind _click_3 (`self.Click`))
  (bind _click_4 (`self.Click`))
  (bind _output (`|GetArrayItem` _click 1))
  (bind _output_2 (`|GetArrayItem` _click))
  (bind _output_3 (`|GetArrayItem` _click_2))
  (bind _output_4 (`|GetArrayItem` _click_2 1))
  (bind _output_5 (`|GetArrayItem` _click_3))
  (bind _output_6 (`|GetArrayItem` _click_3 1))
  (bind _output_7 (`|GetArrayItem` _click_4))
  (bind _output_8 (`|GetArrayItem` _click_4 1))
  (if (> (`KismetArrayLibrary.Array_Length` _click_2) 1)
    (`|ExecutionSequence`
      (:`then_0`
        (`|ExecutionSequence`
          (:`then_0`
            (if (and (== _output_3 "RightMouseButton") (== _output_4 "LeftMouseButton"))
              (set `self.ClickType` "NewEnumerator2" :!label _label)))
          (:`then_1`
            (if (and (== _output_3 "LeftMouseButton") (== _output_4 "RightMouseButton"))
              (goto _label)))))
      (:`then_1`
        (`|ExecutionSequence`
          (:`then_0`
            (if (and (== _output_5 "ThumbMouseButton2") (== _output_6 "LeftMouseButton"))
              (set `self.ClickType` "NewEnumerator4" :!label _label_2)))
          (:`then_1`
            (if (and (== _output_5 "LeftMouseButton") (== _output_6 "ThumbMouseButton2"))
              (goto _label_2)))))
      (:`then_2`
        (`|ExecutionSequence`
          (:`then_0`
            (if (and (== _output_7 "ThumbMouseButton2") (== _output_8 "RightMouseButton"))
              (set `self.ClickType` "NewEnumerator5" :!label _label_3)))
          (:`then_1`
            (if (and (== _output_7 "RightMouseButton") (== _output_8 "ThumbMouseButton2"))
              (goto _label_3)))))
      (:`then_3`
        (`|ExecutionSequence`
          (:`then_0`
            (if (and (== _output_2 "ThumbMouseButton2") (== _output "SpaceBar"))
              (set `self.ClickType` "NewEnumerator6" :!label _label_4)))
          (:`then_1`
            (if (and (== _output_2 "SpaceBar") (== _output "ThumbMouseButton2"))
              (goto _label_4))))))))

(fn `Is Special Key`
  (returns (ReturnValue :type Boolean))
  (`self.InputQueue`)
  (`KismetSystemLibrary.K2_SetTimer` null "DeQueue" 0.2 true)
  (return (`|EnumEquality` (`self.ClickType`) "NewEnumerator7")))

(fn `Is State Action`
  (returns (Result :type Boolean))
  (return (`|EnumEquality` (`self.StateType`) "NewEnumerator1")))

(fn `Is State Idling`
  (returns (Result :type Boolean))
  (return (`|EnumEquality` (`self.StateType`) "NewEnumerator0")))

(fn `Set Current Item`
  (params (`New Item` :type "/Game/Item/BP_Item Object Reference"))
  (returns (Result :type Boolean))
  (set `self.Equip Current Item` `New Item`)
  (return false))

(fn `SetCanMove`
  (params (InCanMove :type Boolean))
  (returns (Result :type Boolean))
  (set `self.CanMove` InCanMove)
  (return false))

(fn `SetStateAction`
  (returns (Result :type Boolean))
  (set `self.StateType` "NewEnumerator1")
  (return false))

(fn `SetStateIdle`
  (returns (Result :type Boolean))
  (set `self.StateType` "NewEnumerator0")
  (return false))

(fn `UserConstructionScript`)